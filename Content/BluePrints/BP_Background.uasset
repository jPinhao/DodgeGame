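; BP_Background is the background actor for a dodge game, doubling as the touch target for restarting after a game over.
; At BeginPlay it scales itself to the viewport size divided by its unscaled box extent and prints the new scale on screen.
; A touch asks DodgeGameMode to change from Game Over to Playing.
; An unconnected camera lookup for ortho width and aspect ratio never runs.
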(event EventActorOnInputTouchBegin
  (params (FingerIndex :type ETouchIndex%20Enum :default "Touch1"))
  (bind _asdodge_game_mode (Utilities|Casting|CastToDodgeGameMode (Game|GetGameMode)))
  (bind _returnvalue (Class|DodgeGameMode|GetGameState _asdodge_game_mode))
  (switch Utilities|FlowControl|Switch|SwitchonEPlayState _returnvalue
    (:EGameOver
      (Class|DodgeGameMode|ChangeGameState _asdodge_game_mode "EPlaying"))))

(event EventBeginPlay
  (bind _returnvalue (Viewport|GetViewportSize))
  (bind _returnvalue_2 (Components|Box|GetUnscaledBoxExtent))
  (bind _returnvalue_3 (Math|Conversions|ToVector(Vector2D) _returnvalue))
  (bind _returnvalue_4 (/ _returnvalue_3 _returnvalue_2))
  (Transformation|SetActorScale3D _returnvalue_4)
  (Development|PrintString (Utilities|String|Append "NewScale: " (Utilities|String|ToString(Vector) _returnvalue_4)) true false))

(fn ConstructionScript)